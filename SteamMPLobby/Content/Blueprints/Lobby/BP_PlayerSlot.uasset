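; BP_PlayerSlot is a lobby slot that shows a character for an assigned player.
; AddPlayer stores the player controller, destroys any existing character and spawns a BP_ThirdPersonCharacter at the slot's Arrow transform.
; It then raises the character by its capsule half-height so it stands on the arrow's position.
; RemovePlayer clears the stored controller and destroys the character, leaving the slot empty.
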(event Custom|Add%20Player
  (params (PC :type Player%20Controller%20Object%20Reference))
  (bind _arrow (Variables|Default|GetArrow))
  (bind _returnvalue (Transformation|GetWorldTransform _arrow))
  (Variables|Default|SetPC PC)
  (bind _selected_character (Variables|Default|GetSelected%20Character)
    (:then
      (Actor|DestroyActor _selected_character))
    (:else
      _))
  (bind _returnvalue_2 (Game|SpawnActorfromClass "/Game/ThirdPerson/Blueprints/BP_ThirdPersonCharacter.BP_ThirdPersonCharacter_C" (Transformation|GetWorldTransform (Variables|Default|GetArrow)) "AlwaysSpawn" "MultiplyWithRoot" 0 0))
  (bind _output_get (Variables|Default|SetSelected%20Character _returnvalue_2))
  (Transformation|SetActorTransform _output_get (Math|Transform|MakeTransform (Math|Vector|MakeVector (.x (.location _returnvalue)) (.y (.location _returnvalue)) (+ (Components|Capsule|GetScaledCapsuleHalfHeight (Variables|/Script/Engine.Character|GetCapsuleComponent _returnvalue_2)) (.z (.location _returnvalue)))) (.rotation _returnvalue) (.scale _returnvalue))))

(event Custom|Remove%20Player
  (Variables|Default|SetPC 0)
  (bind _selected_character (Variables|Default|GetSelected%20Character)
    (:then
      (Actor|DestroyActor _selected_character)
      (Variables|Default|SetPC 0))
    (:else)))

(fn ConstructionScript)